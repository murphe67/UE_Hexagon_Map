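; Game manager that bootstraps a hex-grid, turn-based game and acts as the shared reference hub for its subsystems.
; BeginPlay spawns the pathfinding, hex, turn, roll, effects, enemy, attack and level managers, caches the HUD, then wires up references.
; It places a team 1 character at a hard-coded cube coordinate before initialising the enemy and turn managers; the chaser spawn is disconnected.
; StartGame starts the turn and unlocks the player camera.
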(event EventBeginPlay
  ;[1 1 1] Create Managers
  (CallFunction|SpawnManagers)
  (CallFunction|ConstructReferences)
  ;[1 1 1] Spawn Characters
  (CallFunction|SpawnCharacters)
  (Default|Initialise (Variables|References|GetenemyManagerRef))
  (Default|Initialise (Variables|References|GetturnManagerRef)))

(fn ConstructionScript)

(fn SpawnManagers
  (bind _returnvalue (Game|SpawnActorfromClass (Variables|Classes|GetpathfindingManagerClass) (Math|Transform|MakeTransform "0, 0, 0") "AlwaysSpawn" 0 0))
  (Variables|References|SetpathfindingManagerRef _returnvalue)
  (bind _returnvalue_2 (Game|SpawnActorfromClass (Variables|Classes|GethexManagerClass) (Math|Transform|MakeTransform "0, 0, 0") "AlwaysSpawn" 0 (Variables|Default|GetgenerateAllHexes) (Variables|Default|GetmapRadius) self 0))
  (Variables|References|SethexManagerRef _returnvalue_2)
  (bind _returnvalue_3 (Game|SpawnActorfromClass (Variables|Classes|GetturnManagerClass) (Math|Transform|MakeTransform "0, 0, 0") "AlwaysSpawn" 0 0))
  (Variables|References|SetturnManagerRef _returnvalue_3)
  (bind _returnvalue_4 (Game|SpawnActorfromClass (Variables|Classes|GetrollManagerClass) (Math|Transform|MakeTransform "0, 0, 0") "AlwaysSpawn" 0 0))
  (Variables|References|SetrollManagerRef _returnvalue_4)
  (bind _returnvalue_5 (Game|SpawnActorfromClass (Variables|Classes|GeteffectsManagerClass) (Math|Transform|MakeTransform "0, 0, 0") "Undefined" 0 0))
  (Variables|References|SeteffectsManagerRef _returnvalue_5)
  (bind _returnvalue_6 (Game|SpawnActorfromClass (Variables|Classes|GetenemyManagerClass) (Math|Transform|MakeTransform "0, 0, 0") "AlwaysSpawn" 0 0))
  (Variables|References|SetenemyManagerRef _returnvalue_6)
  (bind _returnvalue_7 (Game|SpawnActorfromClass (Variables|Classes|GetattackManagerClass) (Math|Transform|MakeTransform "0, 0, 0") "AlwaysSpawn" 0 0))
  (Variables|References|SetattackManagerRef _returnvalue_7)
  (bind _ashud_critical_role_bp (Utilities|Casting|CastToHudCriticalRole_BP (HUD|GetHUD (Game|GetPlayerController 0))))
  (Variables|References|SetHUDref _ashud_critical_role_bp)
  (bind _returnvalue_8 (Game|SpawnActorfromClass (Variables|Classes|GetlevelManagerClass) (Math|Transform|MakeTransform "0, 0, 0") "AlwaysSpawn" 0 0))
  (Variables|Default|SetlevelManagerRef _returnvalue_8))

(fn ConstructReferences
  (Default|ConstructReferences (Variables|References|GetrollManagerRef) self)
  (bind _ascritical_role_player_controller (Utilities|Casting|CastToCriticalRole_PlayerController (Game|GetPlayerController 0)))
  (Default|ConstructReferences _ascritical_role_player_controller self)
  (Default|ConstructReferences (Variables|References|GetenemyManagerRef) self)
  (Default|ConstructReferences (Variables|References|GethexManagerRef))
  (Default|ConstructReferences (Variables|References|GetattackManagerRef) self)
  (Default|ConstructReferences (Variables|References|GetturnManagerRef) self))

(fn SpawnCharacters
  (Utilities|FlowControl|Sequence
    (:then_0
      (bind _output_get (LocalVariables|Setx 4))
      (bind _output_get_2 (LocalVariables|Sety 1))
      (bind _output_get_3 (LocalVariables|SettempVector (Math|Vector|MakeVector (Math|Conversions|ToFloat(Integer) _output_get) (Math|Conversions|ToFloat(Integer) _output_get_2) (Math|Conversions|ToFloat(Integer) (- 0 (+ (LocalVariables|Getx) (LocalVariables|Gety)))))))
      (if (.Success (Default|GetHex (Variables|References|GethexManagerRef) _output_get_3))
        (if (not (Variables|/Game/Blueprints/HexMapBlueprints/Hex/Hex_BP.Hex_BP_C|Getoccupied (.Hex (Default|GetHex (Variables|References|GethexManagerRef) _output_get_3))))
          (bind _returnvalue (Game|SpawnActorfromClass (Variables|Classes|GetbaseCharacterClass) (Math|Transform|MakeTransform (Transformation|GetActorLocation (.Hex (Default|GetHex (Variables|References|GethexManagerRef) _output_get_3)))) "Undefined" 0 1 0))
          (Default|ConstructReferences _returnvalue self (.Hex (Default|GetHex (Variables|References|GethexManagerRef) _output_get_3))))))))

(fn StartGame
  (Default|StartTurn (Variables|References|GetturnManagerRef))
  (bind _ascritical_role_player_controller (Utilities|Casting|CastToCriticalRole_PlayerController (Game|GetPlayerController 0)))
  (Variables|/Game/Blueprints/GameBlueprints/CriticalRole_PlayerController.CriticalRole_PlayerController_C|SetcameraLocked _ascritical_role_player_controller false))