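; BaseCharacter_BP is the base character for a turn-based, hex-grid, team game.
; ConstructReferences takes the GameManager and starting hex, initialises the stats, attack, stat-effect and turn components, and occupies that hex.
; It also caches the roll, turn and level managers, binds to the end-turn event and registers the character with its team.
; Activate shows a ring indicator, and Deactivate hides it when passed this character.
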(event EventBeginPlay)

(fn ConstructionScript)

(fn ConstructReferences
  (params (gameManager :type Game%20Manager%20BP%20Object%20Reference) (currentHex :type Hex%20BP%20Object%20Reference))
  (bind _output_get (Variables|References|SetgameManagerRef gameManager))
  (Default|Initialise (Variables|Default|GetCharacterStatsComponent) _output_get)
  (Variables|References|SetrollManagerRef (Variables|/Game/Blueprints/GameBlueprints/GameManager_BP.GameManager_BP_C|GetrollManagerRef _output_get))
  (bind _output_get_2 (Variables|/Game/Blueprints/CharacterBlueprints/MovementComponent.MovementComponent_C|SetcurrentHex (Variables|Default|GetMovementComponent) currentHex))
  (Default|Occupy _output_get_2 self)
  (Default|ConstructReferences (Variables|Default|GetAttackComponent) (Variables|References|GetgameManagerRef))
  (Default|ConstructReferences (Variables|Default|GetStatEffectApplierComponent))
  (Default|ConstructReferences (Variables|Default|GetTurnComponent) (Variables|References|GetgameManagerRef))
  (bind _output_get_3 (Variables|References|SetturnManager (Variables|/Game/Blueprints/GameBlueprints/GameManager_BP.GameManager_BP_C|GetturnManagerRef (Variables|References|GetgameManagerRef))))
  (EventDispatchers|BindEventtoEndTurnEvent _output_get_3 (EventDispatchers|CreateEvent :!event Deactivate))
  (bind _output_get_4 (Variables|References|SetLevelManagerRef (Variables|/Game/Blueprints/GameBlueprints/GameManager_BP.GameManager_BP_C|GetlevelManagerRef (Variables|References|GetgameManagerRef))))
  (Default|AddtoTeam _output_get_4 (Variables|Default|GetTeamNumber) self))

(fn Activate
  (Development|SetHiddeninGame (Variables|Default|Getring) false false))

(fn Deactivate
  (params (ActiveCharacter :type Base%20Character%20BP%20Object%20Reference))
  (if (== ActiveCharacter self)
    (Development|SetHiddeninGame (Variables|Default|Getring) true false)))