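; Manager actor that builds a hexagonal tile map on BeginPlay and answers spatial queries about it.
; Spawns hexes ring by ring on cube coordinates, stores them in a string-keyed map, then initialises those remaining.
; Movement range is a frontier search costed by the pathfinding manager; distance searches reuse the ring generator.
; Visibility passes if any of three line traces, to the target's centre or either side, is unblocked.
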(event EventBeginPlay
  (Spawning|GenerateMap (Variables|Default|GetRadius)))

(fn ConstructionScript)

(fn GenerateMap
  (params (Radius :type Integer))
  (Utilities|FlowControl|Sequence
    (:then_0
      ;[1 1 1] Store the irrational width ratio to reduce overheads
      (Variables|Default|Setsin60Ratio (Math|Trig|Sin(Degrees) 6e+01)))
    (:then_1
      ;[1 1 1] Spawn Centre Hex
      (Spawning|SpawnHexVector "0, 0, 0")
      ;[1 1 1] Create each ring, a hex placed out of bounds will auto self destruct
      (for _index (range 1 Radius)
        (Spawning|GenerateRing _index))
      ;[1 1 1] Calculateneighbours once only the final hexes remain
      (Spawning|Initialise))))

(fn GenerateHexLocation
  (params (CoOrds :type Vector))
  (bind (_x _y _z) (Math|Vector|BreakVector CoOrds))
  (bind _hexsize (Variables|Default|GetHexSize))
  (bind _sin60ratio (Variables|Default|Getsin60Ratio))
  (return (Math|Vector|MakeVector (* (* _hexsize _x) 1.5) (+ (* (* _hexsize _y) _sin60ratio) (* (* (* _hexsize _z) _sin60ratio) -1.0)) 0.0)))

(fn GenerateRing
  (params (RingInput :type Integer))
  (bind _coords (Access|GenerateRingCo-Ords RingInput))
  (for _array_element _coords
    (Spawning|SpawnHexVector _array_element)))

(fn SpawnHexVector
  (params (CoOrds :type Vector))
  (Game|SpawnActorfromClass (Variables|Classes|GetHexClass) (Math|Transform|MakeTransform (Spawning|GenerateHexLocation CoOrds)) "AlwaysSpawn" 0 self CoOrds (Variables|Default|GetgenerateAllHexes) (Variables|References|GetgameManagerRef) 0))

(fn AddHextoArray
  (params (CoOrds :type Vector) (Hex :type Hex%20BP%20Object%20Reference))
  (Utilities|Map|Add (Variables|Default|GetHexMap) (Utilities|String|Append (Utilities|String|ToString(Integer) (Math|Float|Truncate (.x CoOrds))) "." (Utilities|String|ToString(Integer) (Math|Float|Truncate (.y CoOrds))) "." (Utilities|String|ToString(Integer) (Math|Float|Truncate (.z CoOrds)))) Hex))

(fn GetHex
  (params (CoOrds :type Vector))
  (bind _returnvalue (Math|Float|Truncate (.y CoOrds)))
  (bind _returnvalue_2 (Math|Float|Truncate (.x CoOrds)))
  (bind _returnvalue_3 (Math|Float|Truncate (.z CoOrds)))
  (bind _hexmap (Variables|Default|GetHexMap))
  (bind _returnvalue_4 (Utilities|String|ToString(Integer) _returnvalue_2))
  (bind _returnvalue_5 (Utilities|String|ToString(Integer) _returnvalue))
  (bind _returnvalue_6 (Utilities|String|ToString(Integer) _returnvalue_3))
  (bind _returnvalue_7 (Utilities|String|Append _returnvalue_4 "." _returnvalue_5 "." _returnvalue_6))
  (bind (_value _returnvalue_8) (Utilities|Map|Find _hexmap _returnvalue_7))
  (return _value _returnvalue_8))

(fn Initialise
  ;[1 1 1] For each hex in the map
  (bind _keys (Utilities|Map|Keys (Variables|Default|GetHexMap)))
  (for _array_element _keys
    (Default|Initialise (.Value (Utilities|Map|Find (Variables|Default|GetHexMap) _array_element)))))

(fn FindHexesWithinRange
  (params (EnableDifficultTerrain :type Boolean) (StartingHex :type Hex%20BP%20Object%20Reference) (RangeInput :type Integer))
  (bind _hexesvisitablelocal (LocalVariables|GethexesVisitableLocal))
  ;[1 1 1] Store Difficult Terrain
  (LocalVariables|SetenableDifficultTerrainLocal EnableDifficultTerrain)
  ;[1 1 1] Store starting hex
  (bind _output_get (LocalVariables|SetstartingHexLocal StartingHex))
  (LocalVariables|SethexBeingChecked _output_get)
  ;[1 1 1] Store range
  (LocalVariables|SetrangeLocal RangeInput)
  ;[1 1 1] add starting hex to hexes to check
  (Utilities|Array|Add (LocalVariables|GethexesToCheck) (LocalVariables|GethexBeingChecked))
  ;[1 1 1] While there are hexes to check
  (while (> (Utilities|Array|Length (LocalVariables|GethexesToCheck)) 0)
    ;[1 1 1] Get the neighbours of the next hex to check
    (bind _output_get_2 (LocalVariables|SethexBeingChecked (Utilities|Array|Get(acopy) (LocalVariables|GethexesToCheck))))
    ;[1 1 1] For each
    (for _array_element (Variables|/Game/Blueprints/HexMapBlueprints/Hex/Hex_BP.Hex_BP_C|GetNeighbours _output_get_2)
      ;[1 1 1] Store the discovered hex
      (LocalVariables|SetdiscoveredHex _array_element)
      ;[1 1 1] If not already marked as visitable
      (if (not (Utilities|Array|ContainsItem (LocalVariables|GethexesVisitableLocal) (LocalVariables|GetdiscoveredHex)))
        ;[1 1 1] Find how far away the discovered hex is
        (bind (_queue _success _movementcost) (Default|GeneratePath (Variables|References|GetpathfindingManagerRef) (LocalVariables|GetenableDifficultTerrainLocal) (LocalVariables|GetstartingHexLocal) (LocalVariables|GetdiscoveredHex)))
        ;[1 1 1] If within range
        (if _success
          ;[1 1 1] Add it to the hexes within range
          (if (>= (LocalVariables|GetrangeLocal) _movementcost)
            (Utilities|Array|Add (LocalVariables|GethexesVisitableLocal) (LocalVariables|GetdiscoveredHex))
            ;[1 1 1] If there is enough movement left to leave this tile
            (if (> (LocalVariables|GetrangeLocal) _movementcost)
              ;[1 1 1] Add it to the queue to see if it's neighbours are in range
              (if (not (or (Utilities|Array|ContainsItem (LocalVariables|GethexesToCheck) (LocalVariables|GetdiscoveredHex)) (Utilities|Array|ContainsItem (LocalVariables|GetcheckedHexes) (LocalVariables|GetdiscoveredHex))))
                (Utilities|Array|Add (LocalVariables|GethexesToCheck) (LocalVariables|GetdiscoveredHex))))))))
    ;[1 1 1] Remove the hex from the queue to be checked, and mark it as checked
    (Utilities|Array|RemoveItem (LocalVariables|GethexesToCheck) (LocalVariables|GethexBeingChecked))
    (Utilities|Array|Add (LocalVariables|GetcheckedHexes) (LocalVariables|GethexBeingChecked)))
  ;[1 1 1] The hex the character is on is not visitable, as they are already there
  (Utilities|Array|RemoveItem _hexesvisitablelocal (LocalVariables|GetstartingHexLocal))
  (return _hexesvisitablelocal))

(fn ConstructReferences
  (Variables|References|SetpathfindingManagerRef (Variables|/Game/Blueprints/GameBlueprints/GameManager_BP.GameManager_BP_C|GetpathfindingManagerRef (Variables|References|GetgameManagerRef))))

(fn FindHexesWithinDistance
  (params (startingHex :type Hex%20BP%20Object%20Reference) (distance :type Integer))
  (LocalVariables|SetstartingCoOrds (Variables|/Game/Blueprints/HexMapBlueprints/Hex/Hex_BP.Hex_BP_C|GetCoOrds startingHex))
  (for _index (range 1 distance)
    (bind _coords (Access|GenerateRingCo-Ords _index))
    (for _array_element _coords
      (if (.Success (Access|GetHex (+ _array_element (LocalVariables|GetstartingCoOrds))))
        (Utilities|Array|Add (LocalVariables|GethexesWithinDistance) (.Hex (Access|GetHex (+ _array_element (LocalVariables|GetstartingCoOrds))))))))
  (return (LocalVariables|GethexesWithinDistance)))

(fn GenerateRingCo-Ords
  (params (RingInput :type Integer))
  (LocalVariables|SetRing RingInput)
  ;[1 1 1] Begin on hex (0,RingNum,-RingNum)
  (LocalVariables|SetX 0)
  (LocalVariables|SetY (LocalVariables|GetRing))
  (LocalVariables|SetZ (- 0 (LocalVariables|GetRing)))
  ;[1 1 1] Spawn that Hex
  (Utilities|Array|Add (LocalVariables|GetCoOrdsLocal) (Math|Vector|MakeVector (Math|Conversions|ToFloat(Integer) (LocalVariables|GetX)) (Math|Conversions|ToFloat(Integer) (LocalVariables|GetY)) (Math|Conversions|ToFloat(Integer) (LocalVariables|GetZ))))
  ;[1 1 1] Spawn first side of ring
  (while (< (LocalVariables|GetX) (LocalVariables|GetRing))
    (bind _result (Math|Integer|IncrementInt (LocalVariables|GetX))
      (:%20%20
        (bind _result_2 (Math|Integer|DecrementInt (LocalVariables|GetY))
          (:%20%20
            (Utilities|Array|Add (LocalVariables|GetCoOrdsLocal) (Math|Vector|MakeVector (Math|Conversions|ToFloat(Integer) _result) (Math|Conversions|ToFloat(Integer) _result_2) (Math|Conversions|ToFloat(Integer) (LocalVariables|GetZ)))))))))
  ;[1 1 1] Generate second side of ring
  (while (< (Math|Integer|Absolute(Integer) (LocalVariables|GetY)) (LocalVariables|GetRing))
    (bind _result_3 (Math|Integer|IncrementInt (LocalVariables|GetZ))
      (:%20%20
        (bind _result_4 (Math|Integer|DecrementInt (LocalVariables|GetY))
          (:%20%20
            (Utilities|Array|Add (LocalVariables|GetCoOrdsLocal) (Math|Vector|MakeVector (Math|Conversions|ToFloat(Integer) (LocalVariables|GetX)) (Math|Conversions|ToFloat(Integer) _result_4) (Math|Conversions|ToFloat(Integer) _result_3))))))))
  ;[1 1 1] Generate third side of ring
  (while (< (LocalVariables|GetZ) (LocalVariables|GetRing))
    (bind _result_5 (Math|Integer|IncrementInt (LocalVariables|GetZ))
      (:%20%20
        (bind _result_6 (Math|Integer|DecrementInt (LocalVariables|GetX))
          (:%20%20
            (Utilities|Array|Add (LocalVariables|GetCoOrdsLocal) (Math|Vector|MakeVector (Math|Conversions|ToFloat(Integer) _result_6) (Math|Conversions|ToFloat(Integer) (LocalVariables|GetY)) (Math|Conversions|ToFloat(Integer) _result_5))))))))
  ;[1 1 1] Generate fourth side of ring
  (while (< (Math|Integer|Absolute(Integer) (LocalVariables|GetX)) (LocalVariables|GetRing))
    (bind _result_7 (Math|Integer|IncrementInt (LocalVariables|GetY))
      (:%20%20
        (bind _result_8 (Math|Integer|DecrementInt (LocalVariables|GetX))
          (:%20%20
            (Utilities|Array|Add (LocalVariables|GetCoOrdsLocal) (Math|Vector|MakeVector (Math|Conversions|ToFloat(Integer) _result_8) (Math|Conversions|ToFloat(Integer) _result_7) (Math|Conversions|ToFloat(Integer) (LocalVariables|GetZ)))))))))
  ;[1 1 1] Generate fifth side of ring
  (while (< (LocalVariables|GetY) (LocalVariables|GetRing))
    (bind _result_9 (Math|Integer|DecrementInt (LocalVariables|GetZ))
      (:%20%20
        (bind _result_10 (Math|Integer|IncrementInt (LocalVariables|GetY))
          (:%20%20
            (Utilities|Array|Add (LocalVariables|GetCoOrdsLocal) (Math|Vector|MakeVector (Math|Conversions|ToFloat(Integer) (LocalVariables|GetX)) (Math|Conversions|ToFloat(Integer) _result_10) (Math|Conversions|ToFloat(Integer) _result_9))))))))
  ;[1 1 1] Generate sixth side of ring
  (while (< (Math|Integer|Absolute(Integer) (LocalVariables|GetZ)) (- (LocalVariables|GetRing) 1))
    (bind _result_11 (Math|Integer|DecrementInt (LocalVariables|GetZ))
      (:%20%20
        (bind _result_12 (Math|Integer|IncrementInt (LocalVariables|GetX))
          (:%20%20
            (Utilities|Array|Add (LocalVariables|GetCoOrdsLocal) (Math|Vector|MakeVector (Math|Conversions|ToFloat(Integer) _result_12) (Math|Conversions|ToFloat(Integer) (LocalVariables|GetY)) (Math|Conversions|ToFloat(Integer) _result_11))))))))
  (return (LocalVariables|GetCoOrdsLocal)))

(fn FindHexesWithinDIstanceVisible
  (params (Hex :type Hex%20BP%20Object%20Reference) (Distance :type Integer))
  (LocalVariables|SetstartingHex Hex)
  (LocalVariables|SetStartingCoOrdsLocal (Variables|/Game/Blueprints/HexMapBlueprints/Hex/Hex_BP.Hex_BP_C|GetCoOrds Hex))
  (for _index (range 1 Distance)
    (bind _coords (Access|GenerateRingCo-Ords _index))
    (for _array_element _coords
      (if (.Success (Access|GetHex (+ _array_element (LocalVariables|GetStartingCoOrdsLocal))))
        (if (Visibility|IsHexVisible (LocalVariables|GetstartingHex) (.Hex (Access|GetHex (+ _array_element (LocalVariables|GetStartingCoOrdsLocal)))))
          (Utilities|Array|Add (LocalVariables|GethexesWithinDistance) (.Hex (Access|GetHex (+ _array_element (LocalVariables|GetStartingCoOrdsLocal)))))))))
  (return (LocalVariables|GethexesWithinDistance)))

(fn IsHexVisible
  (params (startHex :type Hex%20BP%20Object%20Reference) (endHex :type Hex%20BP%20Object%20Reference))
  (bind _returnvalue (Transformation|GetActorLocation startHex))
  (bind _returnvalue_2 (Transformation|GetActorLocation endHex))
  (bind _hexsize (Variables|Default|GetHexSize))
  (bind _returnvalue_3 (/ _hexsize 1.5))
  (bind _output_get (LocalVariables|SettraceStart (Math|Vector|MakeVector (.x _returnvalue) (.y _returnvalue) (+ (.z _returnvalue) _returnvalue_3))))
  (bind _output_get_2 (LocalVariables|SetcentreVector (Math|Vector|MakeVector (.x _returnvalue_2) (.y _returnvalue_2) (+ (.z _returnvalue_2) _returnvalue_3))))
  (bind _returnvalue_4 (Collision|LineTraceByChannel _output_get _output_get_2 "TraceTypeQuery3" false 0 "None"))
  (bind _returnvalue_5 (Collision|LineTraceByChannel (LocalVariables|GettraceStart) (+ (* (Math|Transform|TransformDirection (Math|Transform|MakeTransform "0, 0, 0" "0,90.000000, 0") (Math|Vector|GetUnitDirection(Vector) (LocalVariables|GettraceStart) (LocalVariables|GetcentreVector))) (/ (Variables|Default|GetHexSize) 4.0)) (LocalVariables|GetcentreVector)) "TraceTypeQuery3" false 0 "None" true "(R=1.000000,G=0.000000,B=0.051694,A=1.000000)" "(R=0.104451,G=1.000000,B=0.000000,A=1.000000)"))
  (bind _returnvalue_6 (Collision|LineTraceByChannel (LocalVariables|GettraceStart) (- (LocalVariables|GetcentreVector) (* (Math|Transform|TransformDirection (Math|Transform|MakeTransform "0, 0, 0" "0,90.000000, 0") (Math|Vector|GetUnitDirection(Vector) (LocalVariables|GettraceStart) (LocalVariables|GetcentreVector))) (/ (Variables|Default|GetHexSize) 4.0))) "TraceTypeQuery3" false 0 "None" true "(R=0.000000,G=0.130012,B=1.000000,A=1.000000)" "(R=0.060412,G=0.000000,B=1.000000,A=1.000000)"))
  (return (Math|Boolean|ORBoolean (not _returnvalue_4) (not _returnvalue_5) (not _returnvalue_6))))

(fn FindDistanceBetweenHexes
  (params (A :type Hex%20BP%20Object%20Reference) (B :type Hex%20BP%20Object%20Reference))
  (bind _coords (Variables|/Game/Blueprints/HexMapBlueprints/Hex/Hex_BP.Hex_BP_C|GetCoOrds A))
  (bind _coords_2 (Variables|/Game/Blueprints/HexMapBlueprints/Hex/Hex_BP.Hex_BP_C|GetCoOrds B))
  (bind (_x _y _z) (Math|Vector|BreakVector _coords))
  (bind (_x_2 _y_2 _z_2) (Math|Vector|BreakVector _coords_2))
  (return (Math|Integer|Max(Integer) (Math|Float|Truncate (Math|Float|Absolute(Float) (- _x _x_2))) (Math|Float|Truncate (Math|Float|Absolute(Float) (- _y _y_2))) (Math|Float|Truncate (Math|Float|Absolute(Float) (- _z _z_2))))))