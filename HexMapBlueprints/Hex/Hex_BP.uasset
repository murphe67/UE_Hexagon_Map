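; Hex tile actor for a hex-grid map that tracks neighbours, movement cost, occupancy and highlight state.
; On construction it sphere-checks for HexOverlapBP actors, registering with the hex manager if found, otherwise destroying itself unless GenerateAllHexes.
; Initialise caches six cube-coordinate neighbours, attaches to the manager and takes movement cost from overlappers, adding rocks for difficult terrain.
; Occupying sets a prohibitive cost; highlight flags pick materials by fixed priority.
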(fn ConstructionScript
  ;[1 1 1] Find hex overlappers
  (bind (_outactors _returnvalue) (Collision|SphereOverlapActors (Transformation|GetActorLocation) 0.1 (Utilities|Array|MakeArray "ObjectTypeQuery1") "/Game/Blueprints/HexMapBlueprints/Overlappers/HexOverlapBP.HexOverlapBP_C"))
  (if _returnvalue
    ;[1 1 1] Add hex to the hex managers array
    (Default|AddHextoArray (Variables|References|GetHexManagerRef) (Variables|Stats|GetCoOrds) self)
    ;[1 1 1] Store overlappers
    (Variables|References|Setoverlappers _outactors)
    (else
      ;[1 1 1] Hexes without an overlapper are removed
      (if (not (Variables|Debug|GetgenerateAllHexes))
        (Actor|DestroyActor)))))

(fn StoreNeighbours
  (bind _neighbours (Variables|Stats|GetNeighbours))
  (bind _hexmanagerref (Variables|References|GetHexManagerRef))
  (bind _coords (Variables|Stats|GetCoOrds))
  (bind (_x _y _z) (Math|Vector|BreakVector _coords))
  (bind _returnvalue (- _x 1.0))
  (bind _returnvalue_2 (- _y 1.0))
  (bind _returnvalue_3 (- _z 1.0))
  (bind _returnvalue_4 (- _y 1.0))
  (bind _returnvalue_5 (- _z 1.0))
  (bind _returnvalue_6 (- _x 1.0))
  (bind _returnvalue_7 (+ _y 1.0))
  (bind _returnvalue_8 (+ _x 1.0))
  (bind _returnvalue_9 (+ _y 1.0))
  (bind _returnvalue_10 (+ _z 1.0))
  (bind _returnvalue_11 (+ _x 1.0))
  (bind _returnvalue_12 (+ _z 1.0))
  (bind (_hex _success) (Default|GetHex _hexmanagerref (Math|Vector|MakeVector _returnvalue _returnvalue_7 _z)))
  (bind (_hex_2 _success_2) (Default|GetHex _hexmanagerref (Math|Vector|MakeVector _x _returnvalue_9 _returnvalue_3)))
  (bind (_hex_3 _success_3) (Default|GetHex _hexmanagerref (Math|Vector|MakeVector _x _returnvalue_4 _returnvalue_10)))
  (bind (_hex_4 _success_4) (Default|GetHex _hexmanagerref (Math|Vector|MakeVector _returnvalue_11 _y _returnvalue_5)))
  (bind (_hex_5 _success_5) (Default|GetHex _hexmanagerref (Math|Vector|MakeVector _returnvalue_6 _y _returnvalue_12)))
  (bind (_hex_6 _success_6) (Default|GetHex _hexmanagerref (Math|Vector|MakeVector _returnvalue_8 _returnvalue_2 _z)))
  ;[1 1 1] For each direction
  (Utilities|FlowControl|Sequence
    (:then_0
      (if _success_2
        ;[1 1 1] Add to neighbours array
        (Utilities|Array|Add _neighbours _hex_2)))
    (:then_1
      (if _success_3
        (Utilities|Array|Add _neighbours _hex_3)))
    (:then_2
      (if _success_4
        (Utilities|Array|Add _neighbours _hex_4)))
    (:then_3
      (if _success_5
        (Utilities|Array|Add _neighbours _hex_5)))
    (:then_4
      (if _success_6
        (Utilities|Array|Add _neighbours _hex_6)))
    (:then_5
      (if _success
        (Utilities|Array|Add _neighbours _hex)))))

(fn Initialise
  (References|StoreNeighbours)
  (Transformation|AttachActorToActor (Variables|References|GetHexManagerRef) "None" "KeepRelative" "KeepRelative" "KeepRelative" true)
  (References|GetDatafromOverlapper))

(fn HighlightPath
  (Variables|Materials|SethighlightedPath true)
  (Materials|UpdateMaterial))

(fn UnhighlightPath
  (Variables|Materials|SethighlightedPath false)
  (Materials|UpdateMaterial))

(fn HighlightinRange
  (Variables|Materials|SethighlightedVisitable true)
  (Materials|UpdateMaterial))

(fn UnhighlightWithinRange
  (Variables|Materials|SethighlightedVisitable false)
  (Materials|UpdateMaterial))

(fn UpdateMaterial
  ;[1 1 1] Path material has highest priority
  (if (Variables|Materials|GethighlightedPath)
    (Rendering|Material|SetMaterial (Variables|Default|GetStaticMesh) 0 (Variables|Materials|GetPathMat))
    (else
      ;[1 1 1] Then the visitable material
      (if (Variables|Materials|GethighlightedVisitable)
        (Rendering|Material|SetMaterial (Variables|Default|GetStaticMesh) 0 (Variables|Materials|GetVisitableMat))
        (elif (Variables|Materials|GethighlightedEnemyInRange)
          (Rendering|Material|SetMaterial (Variables|Default|GetStaticMesh) 0 (Variables|Materials|GetenemyInRangeMat))
          (elif (Variables|Materials|GethighlightedAttackRange)
            (Rendering|Material|SetMaterial (Variables|Default|GetStaticMesh) 0 (Variables|Materials|GetAttackRange))
            (else
              ;[1 1 1] Then default material
              (Rendering|Material|SetMaterial (Variables|Default|GetStaticMesh) 0 (Variables|Materials|GetDefaultMat)))))))))

(fn GetDatafromOverlapper
  ;[1 1 1] For each overlap
  (for _array_element (Variables|References|Getoverlappers)
    ;[1 1 1] Difficult terrain overlap has highest priority
    (bind _asdifficult_terrain_overlap_bp (Utilities|Casting|CastToDifficultTerrainOverlapBP _array_element)
      (:then
        (LocalVariables|Setoverlapper _asdifficult_terrain_overlap_bp)
        (bind _returnvalue (AddComponent|AddStaticMeshComponent false))
        (Components|StaticMesh|SetStaticMesh _returnvalue "/Game/StarterContent/Props/SM_Rock.SM_Rock"))
      (:CastFailed
        ;[1 1 1] Then normal overlap
        (bind _ashex_overlap_bp (Utilities|Casting|CastToHexOverlapBP _array_element))
        (LocalVariables|Setoverlapper _ashex_overlap_bp)))
    ;[1 1 1] Set movement cost, and then store the overlapper's movement cost for reset purposes
    (bind _output_get (Variables|Stats|SetmovementCost (Variables|/Game/Blueprints/HexMapBlueprints/Overlappers/HexOverlapBP.HexOverlapBP_C|GetmovementCost (LocalVariables|Getoverlapper))))
    (Variables|Stats|SetoverlapMovementCost _output_get)))

(fn Occupy
  (params (characterOccupying :type Base%20Character%20BP%20Object%20Reference))
  (Variables|Characters|SetcharacterOccupying characterOccupying)
  (Variables|Stats|SetmovementCost 100000)
  (Variables|Characters|Setoccupied true))

(fn Unoccupy
  (Variables|Stats|SetmovementCost (Variables|Stats|GetoverlapMovementCost))
  (Variables|Characters|Setoccupied false)
  (Variables|Characters|SetcharacterOccupying 0))

(fn HighlightinAttackRange
  (Variables|Materials|SethighlightedAttackRange true)
  (Materials|UpdateMaterial))

(fn UnhighlightinAttackRange
  (Variables|Materials|SethighlightedAttackRange false)
  (Materials|UpdateMaterial))

(fn HighlightEnemyinRange
  (Variables|Materials|SethighlightedEnemyInRange true)
  (Materials|UpdateMaterial))

(fn UnhighlightEnemyinRange
  (Variables|Materials|SethighlightedEnemyInRange false)
  (Materials|UpdateMaterial))