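; Roll manager that resolves D&D-style dice rolls for initiative, attacks and weapon damage.
; A shared RollDice picks a random result for the die type, keeping the higher or lower of two rolls on advantage or disadvantage.
; EffectsManager, taken from the GameManager, supplies advantage, roll multiplier, flat modifier and total multiplier, applied in that order.
; Natural 1 attacks skip modifiers, and damage loops inclusively from zero, rolling one die more than NumberOfDice.
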(fn ConstructionScript)

(fn InitiativeRoll
  (params (Initiative :type Initiative%20Action%20Object%20Reference))
  ;[1 1 1] Find effects on roll
  (bind (_advantageoutput _rollmultiplieroutput _modifieroutput _totalmultiplieroutput) (Default|FindEffectInitiative (Variables|Default|GeteffectsManagerRef) Initiative))
  ;[1 1 1] Roll the dice
  (bind _roll (CallFunction|RollDice "NewEnumerator5" _advantageoutput))
  ;[1 1 1] Modify the roll by effect
  (return (Math|Float|Truncate (* (+ (* _roll _rollmultiplieroutput) (Math|Conversions|ToFloat(Integer) _modifieroutput)) _totalmultiplieroutput))))

(fn ConstructReferences
  (params (gameManager :type Game%20Manager%20BP%20Object%20Reference))
  (Variables|Default|SeteffectsManagerRef (Variables|/Game/Blueprints/GameBlueprints/GameManager_BP.GameManager_BP_C|GeteffectsManagerRef gameManager)))

(fn RollDice
  (params (diceType :type DiceTypeEnumerators%20Enum :default "NewEnumerator0") (advantage :type AdvantageEnumerators%20Enum :default "NewEnumerator0"))
  (Utilities|FlowControl|Sequence
    (:then_0
      ;[1 1 1] Set dice type
      (switch Utilities|FlowControl|Switch|SwitchonDiceTypeEnumerators diceType
        (:NewEnumerator0
          (LocalVariables|SetmaxValue 4))
        (:NewEnumerator1
          (LocalVariables|SetmaxValue 6))
        (:NewEnumerator2
          (LocalVariables|SetmaxValue 8))
        (:NewEnumerator3
          (LocalVariables|SetmaxValue 10))
        (:NewEnumerator4
          (LocalVariables|SetmaxValue 12))
        (:NewEnumerator5
          (LocalVariables|SetmaxValue 20))))
    (:then_1
      ;[1 1 1] Roll dice according to advantage
      (switch Utilities|FlowControl|Switch|SwitchonAdvantageEnumerators advantage
        (:NewEnumerator0
          (Utilities|FlowControl|Sequence
            (:then_0
              (bind _output_get (LocalVariables|SetrollA (Math|Random|RandomIntegerinRange 1 (LocalVariables|GetmaxValue)))))
            (:then_1
              (bind _output_get_2 (LocalVariables|SetrollB (Math|Random|RandomIntegerinRange 1 (LocalVariables|GetmaxValue))))
              (if (< _output_get _output_get_2)
                (LocalVariables|SetrollA (LocalVariables|GetrollB))))))
        (:NewEnumerator1
          (Utilities|FlowControl|Sequence
            (:then_0
              (bind _output_get_3 (LocalVariables|SetrollA (Math|Random|RandomIntegerinRange 1 (LocalVariables|GetmaxValue)))))
            (:then_1
              (bind _output_get_4 (LocalVariables|SetrollB (Math|Random|RandomIntegerinRange 1 (LocalVariables|GetmaxValue))))
              (if (not (< _output_get_3 _output_get_4))
                (LocalVariables|SetrollA (LocalVariables|GetrollB))))))
        (:NewEnumerator2
          (LocalVariables|SetrollA (Math|Random|RandomIntegerinRange 1 (LocalVariables|GetmaxValue))))))
    (:then_2
      ;[1 1 1] Return number
      (return (LocalVariables|GetrollA)))))

(fn AttackRoll
  (params (Attack :type Attack%20Action%20Object%20Reference))
  (bind _output_get (LocalVariables|SetattackLocal Attack))
  ;[1 1 1] Find effects on roll
  (bind (_advantageoutput _rollmultiplieroutput _modifieroutput _totalmultiplieroutput) (Default|FindEffectAttack (Variables|Default|GeteffectsManagerRef) _output_get))
  (bind _roll (CallFunction|RollDice "NewEnumerator5" _advantageoutput))
  ;[1 1 1] Return natural ones
  (if (== _roll 1)
    (return 1)
    (else
      ;[1 1 1] Modify the roll by effect
      (return (Math|Float|Truncate (* (+ (* _roll _rollmultiplieroutput) (Math|Conversions|ToFloat(Integer) _modifieroutput)) _totalmultiplieroutput))))))

(fn DamageRoll
  (params (Attack :type Attack%20Action%20Object%20Reference))
  (bind _output_get (LocalVariables|SetattackLocal Attack))
  ;[1 1 1] Find effects on roll
  (bind (_advantageoutput _rollmultiplieroutput _modifieroutput _totalmultiplieroutput) (Default|FindEffectDamage (Variables|Default|GeteffectsManagerRef) _output_get))
  (Utilities|ForLoop(<) 0 (.NumberOfDice (Utilities|Struct|BreakWeaponStruct (Variables|/Game/Blueprints/EffectsManagerBlueprints/Actions/AttackAction.AttackAction_C|GetWeapon (LocalVariables|GetattackLocal))))
    (:Loop%20Body
      (bind _roll (CallFunction|RollDice (.DiceType (Utilities|Struct|BreakWeaponStruct (Variables|/Game/Blueprints/EffectsManagerBlueprints/Actions/AttackAction.AttackAction_C|GetWeapon (LocalVariables|GetattackLocal)))) _advantageoutput))
      (LocalVariables|SettotalDamage (+ (Math|Conversions|ToFloat(Integer) _roll) (LocalVariables|GettotalDamage))))
    (:Completed
      (Development|PrintString (Utilities|String|Append "Straight damage roll: " (Utilities|String|ToString(Float) (LocalVariables|GettotalDamage))) true true "(R=0.000000,G=0.660000,B=1.000000,A=1.000000)" 2e+01)
      (bind _output_get_2 (LocalVariables|SettotalDamage (* _rollmultiplieroutput (LocalVariables|GettotalDamage))))
      (bind _output_get_3 (LocalVariables|SettotalDamage (+ _output_get_2 (Math|Conversions|ToFloat(Integer) _modifieroutput))))
      (bind _output_get_4 (LocalVariables|SettotalDamage (* _output_get_3 _totalmultiplieroutput)))
      (return (Math|Float|Truncate _output_get_4)))))